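; First-person player controller that sets up Enhanced Input and routes look input to the possessed pawn.
; On BeginPlay it adds the IMC_FPS mapping context and caches the possessed pawn.
; IA_Look passes its value through CalculateSensitivity into the pawn's LookMessage, printing a warning if the cached pawn is invalid.
; The sensitivity scaling math in CalculateSensitivity appears as unused, disconnected nodes.
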(event Input|EnhancedActionEvents|EnhancedInputActionIA_Look
  (params (ActionValue :type Vector%202D%20Structure) (ElapsedSeconds :type Float%20%28double-precision%29) (TriggeredSeconds :type Float%20%28double-precision%29) (InputAction :type Input%20Action%20Object%20Reference :default "/Game/Input/InputActions/IA_Look.IA_Look"))
  (:Triggered
    (bind _possessedpawn (Variables|Default|GetPossessedPawn)
      (:then
        (Class|PlayerActionInterface|Look(Message) _possessedpawn (Utilities|CalculateSensitivity ActionValue)))
      (:else
        (Development|PrintString "PossessedPawn is not valid" true true "(R=1.000000,G=0.000000,B=0.000000,A=1.000000)")))))

(event EventBeginPlay
  (Utilities|FlowControl|Sequence
    (:then_0
      (Utilities|InitInput))
    (:then_1
      (Utilities|SetPossessedPawn))))

(fn ConstructionScript)